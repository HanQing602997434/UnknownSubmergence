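; BP_CustomGameInstance is a custom game instance that holds data meant to persist across levels.
; Events append Ids to a History collection and overwrite the NewGameTimes value.
; Getter functions expose History, NewGameTimes and a TestBeginDialog value, which has no setter in this graph.
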(event EventSaveHistory
  (params (id :type Integer))
  (Utilities|Array|Add (Variables|Default|GetHistory) id))

(event EventSetNewGameTimes
  (params (Times :type Integer))
  (Variables|Default|SetNewGameTimes Times))

(fn GetHistoryData
  (return (Variables|Default|GetHistory)))

(fn GetNewGameTimes
  (return (Variables|Default|GetNewGameTimes)))

(fn GetTestBeginDialog
  (return (Variables|Default|GetTestBeginDialog)))