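; Player controller for a dialogue-driven, visual-novel-style game that opens the start menu and manages the in-game HUD.
; Events forward dialogue, history, save/load, settings, progress and speed commands to HUD sub-widgets, usually recreating the HUD if invalid.
; NextChapter shows a timed transition before rebuilding the HUD.
; SaveGame and LoadGame persist dialogue position and history in BP_SaveGame slots, exchanging history with the GameInstance.
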(event Custom|InGameUIVailid
  (Utilities|IsValid (Variables|Default|GetInGameUI)
    (:Is%20Not%20Valid
      (bind _returnvalue (UserInterface|CreateWidget "/Game/UI/W_PlayerControllerHUD.W_PlayerControllerHUD_C"))
      (bind _output_get (Variables|Default|SetInGameUI _returnvalue))
      (Widget|SetVisibility _output_get "Visible")
      (UserInterface|Viewport|AddtoViewport _output_get 0))))

(event Custom|SetDialog
  (params (DialogID :type Integer))
  (bind _ingameui (Variables|Default|GetInGameUI))
  (bind _w_dialog (Variables|/Game/UI/W_PlayerControllerHUD.W_PlayerControllerHUD_C|GetW_Dialog _ingameui))
  (CallFunction|InGameUIVailid)
  (Default|SetDialogID _w_dialog 0 0 DialogID)
  (Default|NextDialog _w_dialog))

(event EventBeginPlay
  (bind _returnvalue (Game|GetPlayerController 0))
  (bind _returnvalue_2 (UserInterface|CreateWidget "/Game/UI/W_GameStart.W_GameStart_C" _returnvalue))
  (Widget|SetVisibility _returnvalue_2 "Visible")
  (UserInterface|Viewport|AddtoViewport _returnvalue_2 0)
  (Variables|/Script/Engine.PlayerController|SetbShowMouseCursor _returnvalue true))

(event EventCreateGameUI
  (params (Times :type Integer) (Chapter :type Integer) (Dialog :type Integer) (Index :type Integer))
  (bind _returnvalue (UserInterface|CreateWidget "/Game/UI/W_PlayerControllerHUD.W_PlayerControllerHUD_C" self))
  (bind _output_get (Variables|Default|SetInGameUI _returnvalue))
  (Widget|SetVisibility _output_get "Visible")
  (UserInterface|Viewport|AddtoViewport _output_get 0)
  (if (== Dialog -1)
    (bind _dialog (Class|GIInterface|GetTestBeginDialog(Message) (Game|GetGameInstance)))
    (Default|SetDialogID (Variables|/Game/UI/W_PlayerControllerHUD.W_PlayerControllerHUD_C|GetW_Dialog _returnvalue) Times Chapter _dialog)
    (else
      (Default|SetDialogID (Variables|/Game/UI/W_PlayerControllerHUD.W_PlayerControllerHUD_C|GetW_Dialog _returnvalue) Times Chapter Dialog)
      (Default|SetReadIndex (Variables|/Game/UI/W_PlayerControllerHUD.W_PlayerControllerHUD_C|GetW_Dialog _returnvalue) Index)))
  (Utilities|FlowControl|Delay 1.0)
  (Default|FirstShow (Variables|/Game/UI/W_PlayerControllerHUD.W_PlayerControllerHUD_C|GetW_Dialog _returnvalue))
  (Input|SetInputModeGameandUI self 0 "DoNotLock" true))

(event EventShowLoad
  (CallFunction|InGameUIVailid)
  (Widget|SetVisibility (Variables|/Game/UI/W_PlayerControllerHUD.W_PlayerControllerHUD_C|GetW_Load (Variables|Default|GetInGameUI)) "Visible"))

(event EventShowSettings
  (CallFunction|InGameUIVailid)
  (Widget|SetVisibility (Variables|/Game/UI/W_PlayerControllerHUD.W_PlayerControllerHUD_C|GetW_Settings (Variables|Default|GetInGameUI)) "Visible"))

(event EventRemoveGameUI
  (bind _ingameui (Variables|Default|GetInGameUI))
  (Utilities|IsValid _ingameui
    (:Is%20Valid
      (Widget|RemovefromParent _ingameui))))

(event EventHideSave
  (CallFunction|InGameUIVailid)
  (Widget|SetVisibility (Variables|/Game/UI/W_PlayerControllerHUD.W_PlayerControllerHUD_C|GetW_Save (Variables|Default|GetInGameUI)) "Collapsed"))

(event EventSetSaveInfo
  (params (Index :type Integer))
  (CallFunction|InGameUIVailid)
  (Default|SetCover (Variables|/Game/UI/W_Load.W_Load_C|GetW_SaveGame (Variables|/Game/UI/W_PlayerControllerHUD.W_PlayerControllerHUD_C|GetW_Load (Variables|Default|GetInGameUI))) Index))

(event EventShowProgress
  (params (Show? :type Boolean))
  (bind _ingameui (Variables|Default|GetInGameUI))
  (bind _w_circleprogress (Variables|/Game/UI/W_PlayerControllerHUD.W_PlayerControllerHUD_C|GetW_CircleProgress _ingameui))
  (CallFunction|InGameUIVailid)
  (if Show?
    (Widget|SetVisibility _w_circleprogress "Visible")
    (Default|Reset _w_circleprogress)
    (Default|PlayProgressAnim _w_circleprogress)
    (Utilities|FlowControl|Delay 0.5)
    (Widget|SetVisibility _w_circleprogress "Collapsed")
    (else
      (Widget|SetVisibility _w_circleprogress "Collapsed"))))

(event EventSetTextSpeed
  (params (TextSpeed :type Float%20%28single-precision%29))
  (bind _ingameui (Variables|Default|GetInGameUI))
  (bind _output_get (Variables|Default|SetTextSpeed TextSpeed))
  (Utilities|IsValid _ingameui
    (:Is%20Valid
      (Default|SetTextSpeed (Variables|/Game/UI/W_PlayerControllerHUD.W_PlayerControllerHUD_C|GetW_Dialog _ingameui) _output_get))))

(event EventShowHistory
  (CallFunction|InGameUIVailid)
  (Widget|SetVisibility (Variables|/Game/UI/W_PlayerControllerHUD.W_PlayerControllerHUD_C|GetW_History (Variables|Default|GetInGameUI)) "Visible"))

(event EventSetFastSpeed
  (params (FastSpeed :type Float%20%28single-precision%29))
  (bind _ingameui (Variables|Default|GetInGameUI))
  (bind _output_get (Variables|Default|SetFastSpeed FastSpeed))
  (Utilities|IsValid _ingameui
    (:Is%20Valid
      (Default|SetFastSpeed (Variables|/Game/UI/W_PlayerControllerHUD.W_PlayerControllerHUD_C|GetW_Dialog _ingameui) _output_get))))

(event EventSetHistoryUI
  (params (ID :type Integer))
  (bind _ingameui (Variables|Default|GetInGameUI))
  (Utilities|IsValid _ingameui
    (:Is%20Valid
      (Default|SetHistoryUI (Variables|/Game/UI/W_PlayerControllerHUD.W_PlayerControllerHUD_C|GetW_History _ingameui) ID))))

(event EventSetHistory
  (params (History :type Array%20of%20Integers))
  (for _array_element History
    (Class|GIInterface|SaveHistory(Message) (Game|GetGameInstance) _array_element)))

(event EventResetProgress
  (bind _ingameui (Variables|Default|GetInGameUI))
  (Utilities|IsValid _ingameui
    (:Is%20Valid
      (Default|Reset (Variables|/Game/UI/W_PlayerControllerHUD.W_PlayerControllerHUD_C|GetW_CircleProgress _ingameui)))))

(event EventNextChapter
  (params (ChapterID :type Integer))
  (bind _ingameui (Variables|Default|GetInGameUI))
  (Utilities|IsValid _ingameui
    (:Is%20Valid
      (Widget|RemovefromParent _ingameui)
      (bind _returnvalue (UserInterface|CreateWidget "/Game/UI/W_Time.W_Time_C" 0 ChapterID))
      (Variables|Default|SetTimeWidget _returnvalue)
      (Widget|SetVisibility _returnvalue "Visible")
      (UserInterface|Viewport|AddtoViewport _returnvalue 0)
      (Utilities|FlowControl|Delay 3.0)
      (bind _times (Class|GIInterface|GetNewGameTimes(Message) (Game|GetGameInstance)))
      (CallFunction|CreateGameUI _times ChapterID -1))))

(event EventShowMainMenu
  (CallFunction|InGameUIVailid)
  (Widget|RemovefromParent (Variables|Default|GetInGameUI))
  (bind _returnvalue (UserInterface|CreateWidget "/Game/UI/W_GameStart.W_GameStart_C" self))
  (Widget|SetVisibility _returnvalue "Visible")
  (UserInterface|Viewport|AddtoViewport _returnvalue 0))

(event EventHideDialog
  (bind _ingameui (Variables|Default|GetInGameUI))
  (CallFunction|InGameUIVailid)
  (Widget|SetVisibility (Variables|/Game/UI/W_PlayerControllerHUD.W_PlayerControllerHUD_C|GetW_Dialog _ingameui) "Collapsed")
  (Widget|SetVisibility (Variables|/Game/UI/W_PlayerControllerHUD.W_PlayerControllerHUD_C|GetImage_BG _ingameui) "Collapsed"))

(event EventSetFast
  (CallFunction|InGameUIVailid)
  (Default|SetFast (Variables|/Game/UI/W_PlayerControllerHUD.W_PlayerControllerHUD_C|GetW_Dialog (Variables|Default|GetInGameUI)))
  (Variables|Default|SetFast? true))

(event EventCancelFast
  (CallFunction|InGameUIVailid)
  (Default|CancelFast (Variables|/Game/UI/W_PlayerControllerHUD.W_PlayerControllerHUD_C|GetW_Dialog (Variables|Default|GetInGameUI)))
  (Variables|Default|SetFast? false))

(event EventShowSave
  (CallFunction|InGameUIVailid)
  (Widget|SetVisibility (Variables|/Game/UI/W_PlayerControllerHUD.W_PlayerControllerHUD_C|GetW_Save (Variables|Default|GetInGameUI)) "Visible"))

(event EventSetSkip
  (params (Skip :type Boolean))
  (CallFunction|InGameUIVailid)
  (Default|SetFast (Variables|/Game/UI/W_PlayerControllerHUD.W_PlayerControllerHUD_C|GetW_Dialog (Variables|Default|GetInGameUI))))

(event EventShowDialog
  (params (DialogID :type Integer))
  (bind _ingameui (Variables|Default|GetInGameUI))
  (bind _w_dialog (Variables|/Game/UI/W_PlayerControllerHUD.W_PlayerControllerHUD_C|GetW_Dialog _ingameui))
  (CallFunction|InGameUIVailid)
  (Widget|SetVisibility _ingameui "Visible")
  (Widget|SetVisibility _w_dialog "Visible")
  (Default|SetDialogID _w_dialog 0 0 DialogID)
  (Utilities|FlowControl|Delay 0.5)
  (Default|FirstShow _w_dialog))

(event Input|KeyboardEvents|SpaceBar
  (params (Key :type Key%20Structure))
  (:Pressed
    (CallFunction|InGameUIVailid)))

(fn ConstructionScript)

(fn GetFastSpeed
  (return (Variables|Default|GetFastSpeed)))

(fn GetTextSpeed
  (return (Variables|Default|GetTextSpeed)))

(fn LoadGame
  (params (SlotName :type String))
  (bind _returnvalue (SaveGame|DoesSaveGameExist SlotName))
  (if _returnvalue
    (bind _returnvalue_2 (SaveGame|LoadGamefromSlot SlotName))
    (bind _asbp_save_game (Utilities|Casting|CastToBP_SaveGame _returnvalue_2)
      (:then
        (CallFunction|CreateGameUI (Variables|/Game/Blueprint/Framework/BP_SaveGame.BP_SaveGame_C|GetTimes _asbp_save_game) (Variables|/Game/Blueprint/Framework/BP_SaveGame.BP_SaveGame_C|GetChapter _asbp_save_game))
        (CallFunction|SetHistory (Variables|/Game/Blueprint/Framework/BP_SaveGame.BP_SaveGame_C|GetHistory _asbp_save_game))
        (return true (Variables|/Game/Blueprint/Framework/BP_SaveGame.BP_SaveGame_C|GetTimes _asbp_save_game) (Variables|/Game/Blueprint/Framework/BP_SaveGame.BP_SaveGame_C|GetChapter _asbp_save_game) (Variables|/Game/Blueprint/Framework/BP_SaveGame.BP_SaveGame_C|GetDialogID _asbp_save_game) (Variables|/Game/Blueprint/Framework/BP_SaveGame.BP_SaveGame_C|GetReadIndex _asbp_save_game)))
      (:CastFailed
        (Development|PrintString "Cast To BP_SaveGame Failed")
        (return false 0 0 0 0)))
    (else
      (Development|PrintString "不存在该存档")
      (return false 0 0 0 0))))

(fn SaveGame
  (params (SlotName :type String) (Texture :type String))
  (bind _returnvalue (Game|GetGameInstance))
  (bind _ingameui (Variables|Default|GetInGameUI))
  (bind _w_dialog (Variables|/Game/UI/W_PlayerControllerHUD.W_PlayerControllerHUD_C|GetW_Dialog _ingameui))
  (bind _dialog_id (Variables|/Game/UI/W_Dialog.W_Dialog_C|GetDialog_ID _w_dialog))
  (bind _returnvalue_2 (SaveGame|DoesSaveGameExist SlotName))
  (if _returnvalue_2
    (bind _returnvalue_3 (SaveGame|LoadGamefromSlot SlotName))
    (bind _asbp_save_game (Utilities|Casting|CastToBP_SaveGame _returnvalue_3))
    (Variables|/Game/Blueprint/Framework/BP_SaveGame.BP_SaveGame_C|SetTimes _asbp_save_game (Variables|/Game/UI/W_Dialog.W_Dialog_C|GetTimes _w_dialog))
    (Variables|/Game/Blueprint/Framework/BP_SaveGame.BP_SaveGame_C|SetChapter _asbp_save_game (Variables|/Game/UI/W_Dialog.W_Dialog_C|GetChapter _w_dialog))
    (Variables|/Game/Blueprint/Framework/BP_SaveGame.BP_SaveGame_C|SetDialogID _asbp_save_game _dialog_id)
    (Variables|/Game/Blueprint/Framework/BP_SaveGame.BP_SaveGame_C|SetTexture _asbp_save_game Texture)
    (Variables|/Game/Blueprint/Framework/BP_SaveGame.BP_SaveGame_C|SetReadIndex _asbp_save_game (Variables|/Game/UI/W_Dialog.W_Dialog_C|GetReadIndex _w_dialog))
    (bind _data (Class|GIInterface|GetHistoryData(Message) _returnvalue))
    (Variables|/Game/Blueprint/Framework/BP_SaveGame.BP_SaveGame_C|SetHistory _asbp_save_game _data)
    (bind _returnvalue_4 (SaveGame|SaveGametoSlot _asbp_save_game SlotName))
    (if _returnvalue_4
      (Development|PrintString "保存成功")
      (return _returnvalue_4))
    (else
      (bind _returnvalue_5 (SaveGame|CreateSaveGameObject "/Game/Blueprint/Framework/BP_SaveGame.BP_SaveGame_C"))
      (Variables|/Game/Blueprint/Framework/BP_SaveGame.BP_SaveGame_C|SetTimes _returnvalue_5 (Variables|/Game/UI/W_Dialog.W_Dialog_C|GetTimes _w_dialog))
      (Variables|/Game/Blueprint/Framework/BP_SaveGame.BP_SaveGame_C|SetChapter _returnvalue_5 (Variables|/Game/UI/W_Dialog.W_Dialog_C|GetChapter _w_dialog))
      (Variables|/Game/Blueprint/Framework/BP_SaveGame.BP_SaveGame_C|SetDialogID _returnvalue_5 _dialog_id)
      (Variables|/Game/Blueprint/Framework/BP_SaveGame.BP_SaveGame_C|SetTexture _returnvalue_5 Texture)
      (Variables|/Game/Blueprint/Framework/BP_SaveGame.BP_SaveGame_C|SetReadIndex _returnvalue_5 (Variables|/Game/UI/W_Dialog.W_Dialog_C|GetReadIndex _w_dialog))
      (bind _data_2 (Class|GIInterface|GetHistoryData(Message) _returnvalue))
      (Variables|/Game/Blueprint/Framework/BP_SaveGame.BP_SaveGame_C|SetHistory _returnvalue_5 _data_2)
      (bind _returnvalue_6 (SaveGame|SaveGametoSlot _returnvalue_5 SlotName))
      (if _returnvalue_6
        (Development|PrintString "保存成功")
        (return _returnvalue_6)))))